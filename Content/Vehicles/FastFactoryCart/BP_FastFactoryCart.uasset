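; BP_FastFactoryCart is the Blueprint for the Fast Factory Cart vehicle, defining what dismantling it refunds.
; GetDismantleRefund reads the ingredients of Recipe_FastFactoryCart and merges each into the refund as an inventory stack of the same amount, so the refund follows the recipe.
; The event graph holds only disabled default events and the construction script is empty, so this graph adds no other behavior.
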(fn `GetDismantleRefund`
  (params (out_refund :type "Array of InventoryStack Structure (by ref)"))
  (for _array_element (`FGRecipe.GetIngredients` "/FastFactoryCart/Vehicles/FastFactoryCart/Recipe_FastFactoryCart.Recipe_FastFactoryCart_C")
    (bind (_itemclass _amount) (break `ItemAmount` _array_element))
    (`FGInventoryLibrary.MergeInventoryItem` out_refund (`FGInventoryLibrary.MakeInventoryStack` _amount (`FGInventoryLibrary.MakeInventoryItem` _itemclass))))
  (return))

(fn `UserConstructionScript`)